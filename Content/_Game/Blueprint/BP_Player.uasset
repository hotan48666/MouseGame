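; Player character Blueprint for cursor-driven movement, moving toward the point under the mouse while the right mouse button is held.
; A Gate on Tick traces the cursor on the Visibility channel and calls SimpleMoveToLocation every frame it is open.
; Max walk speed switches between running and walking based on distance to the target, and current speed is printed for debugging.
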(event EventBeginPlay
  (Variables|/Script/Engine.PlayerController|SetbShowMouseCursor (Game|GetPlayerController 0) true))

(event EventTick
  (params (DeltaSeconds :type Float%20%28single-precision%29))
  (Utilities|FlowControl|Gate true
    (:Exit
      (CallFunction|MovetoClickedPoint)
      (Development|PrintString (Utilities|String|ToString(Float) (Math|Vector|VectorLength (Transformation|GetVelocity)))))))

(event Input|MouseEvents|RightMouseButton
  (params (Key :type Key%20Structure :default "None"))
  (:Pressed
    (Utilities|FlowControl|Gate true) ; enters at Open
  )
  (:Released
    (Utilities|FlowControl|Gate true) ; enters at Close
  ))

(fn ConstructionScript)

(fn GetDestionationtoMove
  (return (.location (.HitResult (Game|Player|GetHitResultUnderCursorbyChannel (Game|GetPlayerController 0) "TraceTypeQuery1" true)))))

(fn MovetoClickedPoint
  (bind _destionation (CallFunction|GetDestionationtoMove))
  (LocalVariables|SetMoveDestionation _destionation)
  (if (> (Math|Vector|VectorLength (- (LocalVariables|GetMoveDestionation) (Transformation|GetActorLocation))) 1.5e+02)
    (Variables|/Script/Engine.CharacterMovementComponent|SetMaxWalkSpeed (Variables|Character|GetCharacterMovement) 6e+02)
    (else
      (Variables|/Script/Engine.CharacterMovementComponent|SetMaxWalkSpeed (Variables|Character|GetCharacterMovement) 1.5e+02)))
  (AI|Navigation|SimpleMovetoLocation (Game|GetPlayerController 0) (LocalVariables|GetMoveDestionation)))